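; Enemy Blueprint that patrols a looping list of waypoints and chases the player while they are inside its Box trigger.
; A recursive FollowWaypoints event issues AI MoveTo toward either the player or the current waypoint, pausing briefly after each waypoint.
; Box begin and end overlaps toggle MoveToPlayer and immediately re-run FollowWaypoints to switch targets.
; Only successful moves continue the loop, with no handling for failed moves.
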(event OnComponentBeginOverlap(Box)
  (params (OverlappedComponent :type Primitive%20Component%20Object%20Reference) (OtherActor :type Actor%20Object%20Reference) (OtherComp :type Primitive%20Component%20Object%20Reference) (OtherBodyIndex :type Integer) (bFromSweep :type Boolean) (SweepResult :type Hit%20Result%20Structure%20%28by%20ref%29))
  (if (== (Game|GetPlayerCharacter 0) OtherActor)
    (Variables|Default|SetmoveToPlayer true)
    (CallFunction|FollowWaypoints)))

(event OnComponentEndOverlap(Box)
  (params (OverlappedComponent :type Primitive%20Component%20Object%20Reference) (OtherActor :type Actor%20Object%20Reference) (OtherComp :type Primitive%20Component%20Object%20Reference) (OtherBodyIndex :type Integer))
  (if (== (Game|GetPlayerCharacter 0) OtherActor)
    (Variables|Default|SetmoveToPlayer false)
    (CallFunction|FollowWaypoints)))

(event Custom|followWaypoints
  (if (Variables|Default|GetmoveToPlayer)
    (AI|AIMoveTo self "0, 0, 0" (Game|GetPlayerCharacter 0) 5.0 false
      (:OnSuccess
        (CallFunction|FollowWaypoints)))
    (else
      (AI|AIMoveTo self "0, 0, 0" (Utilities|Array|Get(acopy) (Variables|Default|Getwaypoints) (Variables|Default|GetcurrentWaypoint)) 5.0 false
        (:OnSuccess
          (Math|Integer|IncrementInt (Variables|Default|GetcurrentWaypoint)
            (:%20%20
              (if (>= (Variables|Default|GetcurrentWaypoint) (Utilities|Array|Length (Variables|Default|Getwaypoints)))
                (Variables|Default|SetcurrentWaypoint 0))
              (Utilities|FlowControl|Delay 1.0)
              (CallFunction|FollowWaypoints))))))))

(event EventBeginPlay
  (CallFunction|FollowWaypoints))

(fn ConstructionScript)