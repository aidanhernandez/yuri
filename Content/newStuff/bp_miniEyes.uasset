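; A mini-eye enemy Character that chases the player and damages them on contact.
; YESMOVE starts the chase through AIMoveTo, which re-issues itself on each success, while stopMov halts movement and blocks new move requests.
; Sphere overlap with BP_ThirdPersonCharacter calls its Hit function.
; The chase does not start by itself on BeginPlay and does not retry after a failed move.
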(event OnComponentBeginOverlap(Sphere)
  (params (OverlappedComponent :type Primitive%20Component%20Object%20Reference) (OtherActor :type Actor%20Object%20Reference) (OtherComp :type Primitive%20Component%20Object%20Reference) (OtherBodyIndex :type Integer) (bFromSweep :type Boolean) (SweepResult :type Hit%20Result%20Structure%20%28by%20ref%29))
  (bind _asbp_third_person_character (Utilities|Casting|CastToBP_ThirdPersonCharacter OtherActor))
  (Default|Hit _asbp_third_person_character 1))

(event Custom|followPlayer
  (if (not (Variables|Default|GetstopMove))
    (AI|AIMoveTo self "0, 0, 0" (Game|GetPlayerCharacter 0) 1e+01 false
      (:OnSuccess
        (CallFunction|FollowPlayer)))))

(event Custom|YESMOVE
  (Variables|Default|SetstopMove false)
  (CallFunction|FollowPlayer))

(event Custom|stopMov
  (Components|Movement|StopMovementImmediately (Variables|Character|GetCharacterMovement))
  (Variables|Default|SetstopMove true))

(event EventBeginPlay)

(event Collision|EventActorBeginOverlap
  (params (OtherActor :type Actor%20Object%20Reference)))

(event EventTick
  (params (DeltaSeconds :type Float%20%28single-precision%29)))

(fn ConstructionScript)