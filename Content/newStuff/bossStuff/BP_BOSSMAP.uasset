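; Boss map actor that triggers the boss encounter when the player enters the StartFight volume.
; The overlap either starts the battle or calls the player's final boss dialogue, depending on the player's FirstTimeMeetBoss flag, then destroys the trigger.
; Starting the battle activates the boss through the player character, makes StaticMesh1 visible with collision, and sets two rect lights to high intensity.
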(event OnComponentBeginOverlap(startFight)
  (params (OverlappedComponent :type Primitive%20Component%20Object%20Reference) (OtherActor :type Actor%20Object%20Reference) (OtherComp :type Primitive%20Component%20Object%20Reference) (OtherBodyIndex :type Integer) (bFromSweep :type Boolean) (SweepResult :type Hit%20Result%20Structure%20%28by%20ref%29))
  (bind _asbp_third_person_character (Utilities|Casting|CastToBP_ThirdPersonCharacter OtherActor))
  (if (Variables|/Game/ThirdPerson/Blueprints/BP_ThirdPersonCharacter.BP_ThirdPersonCharacter_C|GetfirstTimeMeetBoss _asbp_third_person_character)
    (CallFunction|StartBattle)
    (else
      (Default|FinalBossDIalouge _asbp_third_person_character)))
  (Components|DestroyComponent (Variables|Default|GetstartFight)))

(event Custom|startBattle
  (bind _staticmesh1 (Variables|Default|GetStaticMesh1))
  (bind _asbp_third_person_character (Utilities|Casting|CastToBP_ThirdPersonCharacter (Game|GetPlayerCharacter 0)))
  (Default|ActivateBoss _asbp_third_person_character)
  (Collision|SetCollisionEnabled _staticmesh1 "QueryAndPhysics")
  (Collision|SetCollisionProfileName _staticmesh1 (Variables|Default|GetIn%20Collision%20Profile%20Name) true :!class /Script/Engine.PrimitiveComponent)
  (Development|SetHiddeninGame _staticmesh1 false false)
  (Rendering|Components|Light|SetIntensity (Variables|Default|GetRectLight) 1e+05))

(event EventBeginPlay)

(event Collision|EventActorBeginOverlap
  (params (OtherActor :type Actor%20Object%20Reference)))

(event EventTick
  (params (DeltaSeconds :type Float%20%28single-precision%29)))

(fn ConstructionScript)