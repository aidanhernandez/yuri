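; BP_bossWall is a boss-area wall actor that checks which key items the player carries when they touch its trigger box.
; On Box overlap it casts to BP_ThirdPersonCharacter and loops through InventoryMain, matching entries against the cigarette, sweat and beaker item names.
; Each match sets the corresponding Cig, Sweat or Beaker flag.
; Nothing in this graph reads or resets those flags, or opens the wall.
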(event OnComponentBeginOverlap(Box)
  (params (OverlappedComponent :type Primitive%20Component%20Object%20Reference) (OtherActor :type Actor%20Object%20Reference) (OtherComp :type Primitive%20Component%20Object%20Reference) (OtherBodyIndex :type Integer) (bFromSweep :type Boolean) (SweepResult :type Hit%20Result%20Structure%20%28by%20ref%29))
  (bind _asbp_third_person_character (Utilities|Casting|CastToBP_ThirdPersonCharacter OtherActor))
  (for _array_element (Variables|/Game/ThirdPerson/Blueprints/BP_ThirdPersonCharacter.BP_ThirdPersonCharacter_C|GetinventoryMain _asbp_third_person_character)
    (if (Utilities|Enum|Equal(Enum) _array_element "Cig")
      (Variables|Default|Setcig true)
      (elif (Utilities|Enum|Equal(Enum) _array_element "Sweat")
        (Variables|Default|Setsweat true)
        (elif (Utilities|Enum|Equal(Enum) _array_element "beaker")
          (Variables|Default|Setbeaker true))))))

(event EventBeginPlay)

(event Collision|EventActorBeginOverlap
  (params (OtherActor :type Actor%20Object%20Reference)))

(event EventTick
  (params (DeltaSeconds :type Float%20%28single-precision%29)))

(fn ConstructionScript)