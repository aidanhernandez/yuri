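; Ophelia enemy character that patrols waypoints, chases the player when AI perception senses them, and plays a punch montage on reaching them.
; A self-restarting AIMoveTo loop switches between patrol and chase, with a DoOnce-gated attack applying the hit mid-montage.
; Incoming hits pause movement and scale damage by the player's weapon and a multiplier, then play death or reaction montages.
; The headshot reaction is chosen by weapon (rifle), not hit location.
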(event OnTargetPerceptionUpdated(AIPerception)
  (params (Actor :type Actor%20Object%20Reference) (Stimulus :type AI%20Stimulus%20Structure))
  (if (not (Variables|Default|GetstopMove))
    (Utilities|Casting|CastToBP_ThirdPersonCharacter Actor)
    (if (.bSuccessfullySensed (Utilities|Struct|BreakAIStimulus Stimulus))
      (Variables|Default|SetmoveToPlayer true)
      (else
        (Variables|Default|SetmoveToPlayer false)))
    (CallFunction|FollowWaypoints)))

(event Custom|enemyHit
  (params (mult :type Integer))
  (Variables|Default|SetmoveDis true)
  (Variables|/Script/Engine.CharacterMovementComponent|SetMaxWalkSpeed (Variables|Character|GetCharacterMovement) 0.0)
  (bind (_damage _headshot) (CallFunction|CalcDamageDone mult))
  (Variables|Default|Sethealth (- (Variables|Default|Gethealth) _damage))
  (if (<= (Variables|Default|Gethealth) 0)
    (Collision|SetCollisionEnabled (Variables|Collision|GetCapsuleComponent) "NoCollision")
    (Pawn|Components|CharacterMovement|DisableMovement (Variables|Character|GetCharacterMovement))
    (bind _returnvalue (Animation|PlayAnimMontage "/Game/newStuff/enemyAni/ofelia/OpheliaGetsDead_Montage.OpheliaGetsDead_Montage" 1.0 "None"))
    (Variables|Default|SetDuration _returnvalue)
    (Utilities|FlowControl|Delay (Variables|Default|GetDuration))
    (Variables|/Script/Engine.SkeletalMeshComponent|SetbPauseAnims (Variables|Character|GetMesh) true)
    (else
      (if _headshot
        (Animation|StopAnimMontage 0)
        (bind _returnvalue_2 (Animation|PlayAnimMontage "/Game/newStuff/enemyAni/ofelia/OpheliaGetsHeadshot_Montage.OpheliaGetsHeadshot_Montage" 1.0 "None"))
        (Variables|Default|SetDuration _returnvalue_2)
        (else
          (Animation|StopAnimMontage 0)
          (bind _returnvalue_3 (Animation|PlayAnimMontage "/Game/newStuff/enemyAni/ofelia/OpheliaGetsShot_Montage.OpheliaGetsShot_Montage" 1.0 "None"))
          (Variables|Default|SetDuration _returnvalue_3)))
      (Utilities|FlowControl|Delay (Variables|Default|GetDuration))
      (Variables|/Script/Engine.CharacterMovementComponent|SetMaxWalkSpeed (Variables|Character|GetCharacterMovement) 2e+02)
      (Variables|Default|SetmoveDis false)
      (CallFunction|FollowWaypoints))))

(event Custom|followWaypoints
  (if (not (Variables|Default|GetstopMove))
    (if (not (Variables|Default|GetmoveDis))
      (if (Variables|Default|GetmoveToPlayer)
        (Utilities|FlowControl|Sequence
          (:then_0
            (Variables|Default|SetcurrentWaypoint 0)
            (Variables|Default|SetNewVar true)
            (AI|AIMoveTo self "0, 0, 0" (Game|GetPlayerCharacter 0) 45.0 false
              (:OnSuccess
                (Variables|Default|SethitCharacter true)
                (CallFunction|FollowWaypoints))))
          (:then_1
            (if (Variables|Default|GethitCharacter)
              (Utilities|FlowControl|DoOnce false :!label _label
                (:Completed
                  (bind _returnvalue (Animation|PlayAnimMontage "/Game/newStuff/enemyAni/AniSeq/NicholasPaunch_Montage.NicholasPaunch_Montage" 1.0 "None"))
                  (Utilities|FlowControl|Delay (- (/ _returnvalue 2.0) 0.1))
                  (bind _asbp_third_person_character (Utilities|Casting|CastToBP_ThirdPersonCharacter (Game|GetPlayerCharacter 0)))
                  (Default|Hit _asbp_third_person_character 2)
                  (Utilities|FlowControl|Delay (- (/ _returnvalue 2.0) 0.1))
                  (Variables|Default|SethitCharacter false)
                  (goto _label Reset))))))
        (else
          (if (Variables|Default|GetNewVar)
            (Utilities|FlowControl|Delay 7.0)
            (Variables|Default|SetNewVar false))
          (AI|AIMoveTo self "0, 0, 0" (Utilities|Array|Get(acopy) (Variables|Default|Getwaypoints) (Variables|Default|GetcurrentWaypoint)) 5.0 false
            (:OnSuccess
              (Math|Integer|IncrementInt (Variables|Default|GetcurrentWaypoint)
                (:%20%20
                  (if (>= (Variables|Default|GetcurrentWaypoint) (Utilities|Array|Length (Variables|Default|Getwaypoints)))
                    (Variables|Default|SetcurrentWaypoint 0))
                  (Utilities|FlowControl|Delay 1.0)
                  (CallFunction|FollowWaypoints))))))))))

(event Custom|YESMOVE
  (Variables|Default|SetstopMove false))

(event Custom|stopMov
  (Components|Movement|StopMovementImmediately (Variables|Character|GetCharacterMovement))
  (Variables|Default|SetstopMove true))

(event EventBeginPlay
  (Utilities|FlowControl|Delay 0.2)
  (Variables|Default|SetmoveToPlayer false)
  (CallFunction|FollowWaypoints))

(fn ConstructionScript)

(fn CalcDamageDone
  (params (mult :type Integer))
  (bind _asbp_third_person_character (Utilities|Casting|CastToBP_ThirdPersonCharacter (Game|GetPlayerCharacter 0)))
  (switch string (Variables|/Game/ThirdPerson/Blueprints/BP_ThirdPersonCharacter.BP_ThirdPersonCharacter_C|Getequipment _asbp_third_person_character)
    (:"pistol"
      (Variables|Default|SetdamageDone 1)
      (LocalVariables|SetNewLocalVar false))
    (:"rifle"
      (Variables|Default|SetdamageDone 2)
      (LocalVariables|SetNewLocalVar true)))
  (bind _output_get (Variables|Default|SetdamageDone (* (Variables|Default|GetdamageDone) mult)))
  (return _output_get (LocalVariables|GetNewLocalVar)))