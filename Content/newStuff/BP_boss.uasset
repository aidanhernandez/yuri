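; Eye boss with four tentacles that creeps toward a waypoint, dragging a map mesh along, while tracking the player sideways.
; A random timer picks a beam, charge or mini-eye spawn, each telegraphed by a light timeline.
; Hits destroy tentacles, exposing the main eye, with rifles counting double and only rifle hits checking eye defeat.
; Defeat clears mini-eyes, flies the boss upward, destroys its meshes, fades out and triggers the player's ending.
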(event OnComponentBeginOverlap(damageCollison)
  (params (OverlappedComponent :type Primitive%20Component%20Object%20Reference) (OtherActor :type Actor%20Object%20Reference) (OtherComp :type Primitive%20Component%20Object%20Reference) (OtherBodyIndex :type Integer) (bFromSweep :type Boolean) (SweepResult :type Hit%20Result%20Structure%20%28by%20ref%29))
  (bind _asbp_third_person_character (Utilities|Casting|CastToBP_ThirdPersonCharacter OtherActor))
  (Default|Hit _asbp_third_person_character 3))

(event OnComponentBeginOverlap(Cube)
  (params (OverlappedComponent :type Primitive%20Component%20Object%20Reference) (OtherActor :type Actor%20Object%20Reference) (OtherComp :type Primitive%20Component%20Object%20Reference) (OtherBodyIndex :type Integer) (bFromSweep :type Boolean) (SweepResult :type Hit%20Result%20Structure%20%28by%20ref%29))
  (bind _asbp_third_person_character (Utilities|Casting|CastToBP_ThirdPersonCharacter OtherActor))
  (Default|Hit _asbp_third_person_character 3))

(event Custom|initiateBossFight
  (CallFunction|CoolEyeGlow)
  (Variables|Default|SetstopMove false)
  (CallFunction|Follow 0.0)
  (Utilities|FlowControl|Delay 2.0)
  (bind _output_get (Variables|Default|SetrandomWait (Math|Random|RandomFloatinRange 5.0 1e+01)))
  (CallFunction|RandomAttack _output_get))

(event Custom|BeamAttack
  (bind _asbp_third_person_character (Utilities|Casting|CastToBP_ThirdPersonCharacter (Game|GetPlayerCharacter 0)))
  (Variables|Default|SetAs%20BP%20Third%20Person%20Character _asbp_third_person_character)
  (Class|NiagaraComponent|SetAsset (Variables|Default|GetNiagara) "/Game/newStuff/bossStuff/beam/Beam.Beam" true)
  (Audio|PlaySound2D "/Game/audioFiles/Laser.Laser" 1.0 1.0 0.0 0 0)
  (bind _newtrack_0 (Timeline|Timeline PlayFromStart)
    (:Update
      (Rendering|Components|Light|SetIntensity (Variables|Default|GetPointLight) (Math|Float|Lerp 5e+03 1e+05 _newtrack_0)))
    (:Finished
      (if (not (Variables|Default|GetstopMove))
        (Variables|Default|SetstopMoveInv true)
        (Default|CameraShakeBeam (Variables|Default|GetAs%20BP%20Third%20Person%20Character) 0.0)
        (Components|Activation|Activate (Variables|Default|GetNiagara) false)
        (Variables|Default|SetIn%20Collision%20Profile%20Name "OverlapAll")
        (Collision|SetCollisionProfileName (Variables|Default|GetCube) (Variables|Default|GetIn%20Collision%20Profile%20Name) true :!class /Script/Engine.PrimitiveComponent)
        (Rendering|Components|Light|SetIntensity (Variables|Default|GetPointLight) 5e+03)
        (Utilities|FlowControl|Delay 3.0)
        (Class|NiagaraComponent|SetAsset (Variables|Default|GetNiagara) "/Game/newStuff/bossStuff/beam/empty.empty" true)
        (Variables|Default|SetIn%20Collision%20Profile%20Name "NoCollision")
        (Collision|SetCollisionProfileName (Variables|Default|GetCube) (Variables|Default|GetIn%20Collision%20Profile%20Name) true :!class /Script/Engine.PrimitiveComponent)
        (Variables|Default|SetstopMoveInv false)
        (CallFunction|Follow 0.0)
        (bind _output_get (Variables|Default|SetrandomWait (Math|Random|RandomFloatinRange 5.0 1e+01)))
        (CallFunction|RandomAttack _output_get)))))

(event Custom|flyAway
  (Variables|Default|Setbye true)
  (bind _asbp_third_person_character (Utilities|Casting|CastToBP_ThirdPersonCharacter (Game|GetPlayerCharacter 0)))
  (Default|FinalMusic _asbp_third_person_character))

(event Custom|CustomEvent
  (bind _mainbody (Variables|Default|GetmainBody))
  (Components|Activation|Activate (Variables|Default|GetNiagara1) false)
  (Audio|PlaySound2D "/Game/audioFiles/BossDeath.BossDeath" 1.0 1.0 0.0 0 0)
  (Utilities|FlowControl|Delay 3.0)
  (Utilities|IsValid _mainbody
    (:Is%20Valid
      (Components|DestroyComponent _mainbody))
    (:Is%20Not%20Valid
      _))
  (Utilities|FlowControl|Delay 1.0)
  (Utilities|FlowControl|Delay 1.0)
  (bind _returnvalue (UserInterface|CreateWidget "/Game/newStuff/Wibget/fadeToblackNoText.fadeToblackNoText_C"))
  (UserInterface|Viewport|AddtoViewport _returnvalue 0)
  (Utilities|FlowControl|Delay 3.0)
  (bind _asbp_third_person_character (Utilities|Casting|CastToBP_ThirdPersonCharacter (Game|GetPlayerCharacter 0)))
  (Default|LastOnefortheFans _asbp_third_person_character))

(event Custom|follow
  (params (NewParam :type Float%20%28double-precision%29))
  (bind _waypoint (Variables|Default|GetwayPoint))
  (bind _capsulecomponent (Variables|Collision|GetCapsuleComponent))
  (bind _returnvalue (Transformation|GetWorldLocation _capsulecomponent))
  (bind _billboard (Variables|/Game/newStuff/bluePrint/BP_Waypoint.BP_Waypoint_C|GetBillboard _waypoint))
  (bind _returnvalue_2 (Transformation|GetWorldLocation _billboard))
  (if (not (Variables|Default|GetstopMove))
    (if (not (Variables|Default|GetstopMoveInv))
      (Transformation|SetActorLocation (Math|Vector|MakeVector (Math|Interpolation|FInterpTo (.x _returnvalue) (.x _returnvalue_2) NewParam 0.0063) (Math|Interpolation|FInterpTo (.y _returnvalue) (.y (Transformation|GetWorldLocation (Variables|/Script/Engine.Character|GetCapsuleComponent (Game|GetPlayerCharacter 0)))) NewParam 1.0) (.z _returnvalue)) false false)
      (bind _outactors (Actor|GetAllActorsOfClass "/Game/newStuff/bossStuff/BP_BOSSMAP.BP_BOSSMAP_C"))
      (Transformation|SetWorldLocation (Variables|/Game/newStuff/bossStuff/BP_BOSSMAP.BP_BOSSMAP_C|GetStaticMesh1 (Utilities|Array|Get(acopy) _outactors)) (Math|Vector|MakeVector (Math|Interpolation|FInterpTo (.x (Transformation|GetWorldLocation (Variables|/Game/newStuff/bossStuff/BP_BOSSMAP.BP_BOSSMAP_C|GetStaticMesh1 (Utilities|Array|Get(acopy) _outactors)))) (.x _returnvalue_2) NewParam 0.0063) (.y (Transformation|GetWorldLocation (Variables|/Game/newStuff/bossStuff/BP_BOSSMAP.BP_BOSSMAP_C|GetStaticMesh1 (Utilities|Array|Get(acopy) _outactors)))) (.z (Transformation|GetWorldLocation (Variables|/Game/newStuff/bossStuff/BP_BOSSMAP.BP_BOSSMAP_C|GetStaticMesh1 (Utilities|Array|Get(acopy) _outactors))))) false false))))

(event Custom|YESMOVE
  (Variables|Default|SetstopMoveInv false))

(event Custom|stopMov
  (Components|Movement|StopMovementImmediately (Variables|Character|GetCharacterMovement))
  (Variables|Default|SetstopMoveInv true))

(event Custom|randomAttack
  (params (NewParam :type Float%20%28double-precision%29))
  (Utilities|Time|SetTimerbyEvent (delegate Custom|waitOver) NewParam))

(event Custom|waitOver
  (if (not (Variables|Default|GetstopMove))
    (switch int (Math|Random|RandomIntegerinRange 1 3)
      (:1
        (CallFunction|BeamAttack))
      (:2
        (CallFunction|Charge))
      (:3
        (CallFunction|SpawnMiniEyes)))))

(event Custom|spawnMiniEyes
  (Variables|Default|SetspawnPoints (Utilities|Array|MakeArray (Variables|Default|GetStaticMesh1) (Variables|Default|GetStaticMesh2) (Variables|Default|GetStaticMesh3) (Variables|Default|GetStaticMesh4)))
  (Variables|Default|SetnumberOfEyes 0)
  (bind _newtrack_0 (Timeline|Timeline_1 PlayFromStart)
    (:Update
      (Rendering|Components|Light|SetLightColor (Variables|Default|GetPointLight) (Math|Color|Lerp(LinearColor) "(R=0.333333,G=1.000000,B=0.980392,A=1.000000)" "(R=0.000000,G=1.000000,B=0.059587,A=1.000000)" _newtrack_0) true)
      (Rendering|Components|Light|SetIntensity (Variables|Default|GetPointLight) (Math|Float|Lerp 5e+03 1e+05 _newtrack_0)))
    (:Finished
      (if (not (Variables|Default|GetstopMove))
        (while (< (Variables|Default|GetnumberOfEyes) (Utilities|Array|Length (Variables|Default|GetspawnPoints)))
          (bind _returnvalue (Game|SpawnActorfromClass "/Game/newStuff/bp_miniEyes.bp_miniEyes_C" (Math|Transform|MakeTransform (Transformation|GetWorldLocation (Utilities|Array|Get(acopy) (Variables|Default|GetspawnPoints) (Variables|Default|GetnumberOfEyes))) "0, 0, 0" "1.000000,1.000000,1.000000") "Undefined" "MultiplyWithRoot" 0 0))
          (Math|Integer|IncrementInt (Variables|Default|GetnumberOfEyes)
            (:%20%20
              (Default|FollowPlayer _returnvalue))))
        (Rendering|Components|Light|SetLightColor (Variables|Default|GetPointLight) "(R=0.333333,G=1.000000,B=0.980392,A=1.000000)" true)
        (Rendering|Components|Light|SetIntensity (Variables|Default|GetPointLight) 5e+03)
        (bind _output_get (Variables|Default|SetrandomWait (Math|Random|RandomFloatinRange 5.0 1e+01)))
        (CallFunction|RandomAttack _output_get)))))

(event Custom|Charge
  (bind _charactermovement (Variables|Character|GetCharacterMovement))
  (bind _capsulecomponent (Variables|Collision|GetCapsuleComponent))
  (bind _returnvalue (Transformation|GetWorldLocation _capsulecomponent))
  (bind _newtrack_0 (Timeline|Timeline_0 PlayFromStart)
    (:Update
      (Rendering|Components|Light|SetLightColor (Variables|Default|GetPointLight) (Math|Color|Lerp(LinearColor) "(R=0.333333,G=1.000000,B=0.980392,A=1.000000)" "(R=1.000000,G=0.000000,B=0.035295,A=1.000000)" _newtrack_0) true)
      (Rendering|Components|Light|SetIntensity (Variables|Default|GetPointLight) (Math|Float|Lerp 5e+03 1e+05 _newtrack_0)))
    (:Finished
      (if (not (Variables|Default|GetstopMove))
        (Variables|Default|SetstopMoveInv true)
        (Variables|Default|SetlastLocation (Transformation|GetActorLocation))
        (Variables|/Script/Engine.CharacterMovementComponent|SetMaxAcceleration _charactermovement 3e+03)
        (Variables|/Script/Engine.CharacterMovementComponent|SetMaxFlySpeed _charactermovement 3e+03)
        (AI|AIMoveTo self (Math|Vector|MakeVector (.x (Transformation|GetWorldLocation (Variables|/Script/Engine.Character|GetCapsuleComponent (Game|GetPlayerCharacter 0)))) (.y _returnvalue) (.z _returnvalue)) 0 1e+01 false
          (:OnSuccess
            (Rendering|Components|Light|SetLightColor (Variables|Default|GetPointLight) "(R=0.333333,G=1.000000,B=0.980392,A=1.000000)" true)
            (Rendering|Components|Light|SetIntensity (Variables|Default|GetPointLight) 5e+03)
            (Variables|/Script/Engine.CharacterMovementComponent|SetMaxFlySpeed (Variables|Character|GetCharacterMovement) 5e+02)
            (AI|AIMoveTo self (Variables|Default|GetlastLocation) 0 1e+01 false
              (:OnSuccess
                (Variables|/Script/Engine.CharacterMovementComponent|SetMaxFlySpeed (Variables|Character|GetCharacterMovement) 6e+02)
                (Variables|Default|SetstopMoveInv false)
                (CallFunction|Follow 0.0)
                (bind _output_get (Variables|Default|SetrandomWait (Math|Random|RandomFloatinRange 5.0 1e+01)))
                (CallFunction|RandomAttack _output_get)))))))))

(event Custom|coolEyeGlow
  (bind _newtrack_0 (Timeline|Timeline_2 PlayFromStart)
    (:Update
      (Rendering|Components|Light|SetIntensity (Variables|Default|GetPointLight) (Math|Float|Lerp 0.0 5e+03 _newtrack_0))
      (Rendering|Components|Light|SetIntensity (Variables|Default|GetPointLight1) (Math|Float|Lerp 0.0 4e+02 _newtrack_0)))))

(event EventTick
  (params (DeltaSeconds :type Float%20%28single-precision%29))
  (bind _capsulecomponent (Variables|Collision|GetCapsuleComponent))
  (bind _returnvalue (Transformation|GetWorldLocation _capsulecomponent))
  (Variables|Default|SetDelta%20Seconds DeltaSeconds)
  (if (Variables|Default|GetstopMove)
    (if (Variables|Default|Getbye)
      (Transformation|SetActorLocation (Math|Vector|MakeVector (.x _returnvalue) (.y _returnvalue) (Math|Interpolation|FInterpTo (.z _returnvalue) (.z (Transformation|GetWorldLocation (Variables|/Game/newStuff/bluePrint/BP_Waypoint.BP_Waypoint_C|GetBillboard (Variables|Default|GetflyAwau)))) (Variables|Default|GetDelta%20Seconds) 0.1)) false false)
      (Utilities|FlowControl|Delay 2.0)
      (Variables|Default|Setbye false)
      (CallFunction|CustomEvent))
    (else
      (Transformation|SetActorRotation "0.000000,180.000000,0.000000")
      (if (not (Variables|Default|GetstopMoveInv))
        (CallFunction|Follow DeltaSeconds)))))

(fn ConstructionScript)

(fn TenticleHit
  (params (NewParam :type Primitive%20Component%20Object%20Reference))
  (bind _hittenticle_0 (Variables|Default|GethitTenticle_0))
  (bind _hittenticle_1 (Variables|Default|GethitTenticle_1))
  (bind _hittenticle_2 (Variables|Default|GethitTenticle_2))
  (bind _hittenticle_3 (Variables|Default|GethitTenticle_3))
  (bind _maineyehit (Variables|Default|GetmainEyeHit))
  (bind _asbp_third_person_character (Utilities|Casting|CastToBP_ThirdPersonCharacter (Game|GetPlayerCharacter 0)))
  (Variables|Default|SetEquipment (Variables|/Game/ThirdPerson/Blueprints/BP_ThirdPersonCharacter.BP_ThirdPersonCharacter_C|Getequipment _asbp_third_person_character))
  (if (== NewParam (Variables|Default|GetSphere))
    (Math|Integer|IncrementInt _hittenticle_0
      (:%20%20
        (if (Utilities|Enum|Equal(Enum) (Variables|Default|GetEquipment) "\"rifle\"")
          (Math|Integer|IncrementInt _hittenticle_0
            (:%20%20
              _)))
        (Variables|Default|SettentIntHit _hittenticle_0)
        (Variables|Default|SetsetTentNum "1")
        (CallFunction|CheckDestruction (Variables|Default|GettentIntHit) (Variables|Default|GetsetTentNum) :!label _label)))
    (elif (== NewParam (Variables|Default|GetSphere1))
      (Math|Integer|IncrementInt _hittenticle_1
        (:%20%20
          (if (Utilities|Enum|Equal(Enum) (Variables|Default|GetEquipment) "\"rifle\"")
            (Math|Integer|IncrementInt _hittenticle_1
              (:%20%20
                _)))
          (Variables|Default|SettentIntHit _hittenticle_1)
          (Variables|Default|SetsetTentNum "2")
          (goto _label)))
      (elif (== NewParam (Variables|Default|GetSphere2))
        (Math|Integer|IncrementInt _hittenticle_2
          (:%20%20
            (if (Utilities|Enum|Equal(Enum) (Variables|Default|GetEquipment) "\"rifle\"")
              (Math|Integer|IncrementInt _hittenticle_2
                (:%20%20
                  _)))
            (Variables|Default|SettentIntHit _hittenticle_2)
            (Variables|Default|SetsetTentNum "3")
            (goto _label)))
        (elif (== NewParam (Variables|Default|GetSphere3))
          (Math|Integer|IncrementInt _hittenticle_3
            (:%20%20
              (if (Utilities|Enum|Equal(Enum) (Variables|Default|GetEquipment) "\"rifle\"")
                (Math|Integer|IncrementInt _hittenticle_3
                  (:%20%20
                    _)))
              (Variables|Default|SettentIntHit _hittenticle_3)
              (Variables|Default|SetsetTentNum "4")
              (goto _label)))
          (elif (== NewParam (Variables|Default|GetbossHitRadius))
            (if (Variables|Default|GettenticleDestroyed_0)
              (if (Variables|Default|GettenticleDestroyed_1)
                (if (Variables|Default|GettenticleDestroyed_2)
                  (if (Variables|Default|GettenticleDestroyed_3)
                    (Math|Integer|IncrementInt _maineyehit
                      (:%20%20
                        (if (Utilities|Enum|Equal(Enum) (Variables|Default|GetEquipment) "\"rifle\"")
                          (Math|Integer|IncrementInt _maineyehit
                            (:%20%20
                              (bind _output_get (Variables|Default|SettentIntHit _maineyehit))
                              (bind _output_get_2 (Variables|Default|SetsetTentNum "main"))
                              (CallFunction|CheckDestruction _output_get _output_get_2))))))))))))))))

(fn CheckDestruction
  (params (NewParam :type Integer) (NewParam1 :type String))
  (if (Utilities|Enum|Equal(Enum) NewParam1 "main")
    (if (>= NewParam 5)
      (Variables|Default|SetstopMove true)
      (bind _outactors (Actor|GetAllActorsOfClass "/Game/newStuff/bp_miniEyes.bp_miniEyes_C"))
      (for _array_element _outactors
        (Actor|DestroyActor _array_element))
      (CallFunction|FlyAway))
    (elif (>= NewParam 2)
      (switch string NewParam1
        (:1
          (Variables|Default|SettenticleDestroyed_0 true)
          (Components|DestroyComponent (Variables|Default|GetSphere)))
        (:2
          (Variables|Default|SettenticleDestroyed_1 true)
          (Components|DestroyComponent (Variables|Default|GetSphere1)))
        (:3
          (Variables|Default|SettenticleDestroyed_2 true)
          (Components|DestroyComponent (Variables|Default|GetSphere2)))
        (:4
          (Variables|Default|SettenticleDestroyed_3 true)
          (Components|DestroyComponent (Variables|Default|GetSphere3)))))))