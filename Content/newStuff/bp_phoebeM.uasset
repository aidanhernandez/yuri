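; Phoebe actor with a capsule and mesh that triggers a blackout sequence when the car hits it.
; Capsule overlap with BP_car destroys the car and immediately shows a Black widget.
; A DoOnce then runs a delayed sequence that adds a FadeToblack widget, later removes Black and destroys this actor.
; A physics-simulation call on the mesh is left unconnected.
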(event OnComponentBeginOverlap(CapsuleComponent)
  (params (OverlappedComponent :type Primitive%20Component%20Object%20Reference) (OtherActor :type Actor%20Object%20Reference) (OtherComp :type Primitive%20Component%20Object%20Reference) (OtherBodyIndex :type Integer) (bFromSweep :type Boolean) (SweepResult :type Hit%20Result%20Structure%20%28by%20ref%29))
  (bind _asbp_car (Utilities|Casting|CastToBP_car OtherActor))
  (Actor|DestroyActor _asbp_car)
  (bind _returnvalue (UserInterface|CreateWidget "/Game/newStuff/Wibget/black.black_C"))
  (UserInterface|Viewport|AddtoViewport _returnvalue 0)
  (Utilities|FlowControl|DoOnce false
    (:Completed
      (Utilities|FlowControl|Delay 3.0)
      (bind _returnvalue_2 (UserInterface|CreateWidget "/Game/newStuff/Wibget/fadeToblack.fadeToblack_C"))
      (UserInterface|Viewport|AddtoViewport _returnvalue_2 0)
      (Utilities|FlowControl|Delay 3.0)
      (Widget|RemovefromParent _returnvalue)
      (Actor|DestroyActor))))

(fn ConstructionScript)