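; BP_unlockedDoor is a door that toggles open and closed through its openDoor event.
; Based on DoorOpen, one timeline plays forward or another in reverse, lerping the door's yaw between 0 and -90 degrees and updating the flag each tick.
; The OpenDoorRadius overlap writes a string tag to BP_ThirdPersonCharacter's InDoorRadius, marking it "unlockedDoor" on entry and "none" on exit.
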(event OnComponentBeginOverlap(openDoorRadius)
  (params (OverlappedComponent :type Primitive%20Component%20Object%20Reference) (OtherActor :type Actor%20Object%20Reference) (OtherComp :type Primitive%20Component%20Object%20Reference) (OtherBodyIndex :type Integer) (bFromSweep :type Boolean) (SweepResult :type Hit%20Result%20Structure%20%28by%20ref%29))
  (bind _asbp_third_person_character (Utilities|Casting|CastToBP_ThirdPersonCharacter OtherActor))
  (Variables|/Game/ThirdPerson/Blueprints/BP_ThirdPersonCharacter.BP_ThirdPersonCharacter_C|SetinDoorRadius _asbp_third_person_character "\"unlockedDoor\""))

(event OnComponentEndOverlap(openDoorRadius)
  (params (OverlappedComponent :type Primitive%20Component%20Object%20Reference) (OtherActor :type Actor%20Object%20Reference) (OtherComp :type Primitive%20Component%20Object%20Reference) (OtherBodyIndex :type Integer))
  (bind _asbp_third_person_character (Utilities|Casting|CastToBP_ThirdPersonCharacter OtherActor))
  (Variables|/Game/ThirdPerson/Blueprints/BP_ThirdPersonCharacter.BP_ThirdPersonCharacter_C|SetinDoorRadius _asbp_third_person_character "\"none\""))

(event Custom|openDoor
  (if (Variables|Default|GetdoorOpen?)
    (bind _doorfloat (Timeline|Timeline ReverseFromEnd)
      (:Update
        (Transformation|SetRelativeRotation (Variables|Default|Getdoor) (Math|Rotator|MakeRotator 0.0 0.0 (Math|Float|Lerp 0.0 -9e+01 _doorfloat)) false false)
        (Variables|Default|SetdoorOpen? false)))
    (else
      (bind _doorfloat_2 (Timeline|Timeline_1 PlayFromStart)
        (:Update
          (Transformation|SetRelativeRotation (Variables|Default|Getdoor) (Math|Rotator|MakeRotator 0.0 0.0 (Math|Float|Lerp 0.0 -9e+01 _doorfloat_2)) false false)
          (Variables|Default|SetdoorOpen? true))))))

(fn ConstructionScript)