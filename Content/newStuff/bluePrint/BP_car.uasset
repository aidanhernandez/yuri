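; BP_car is a car actor that drives itself to a single Waypoint actor once startMov is called.
; startMov sets a flag that lets Tick spin two wheel pairs in opposite roll directions at a constant rate.
; While the flag is set, Tick also eases the car toward the waypoint with VInterpTo, without sweeping or changing the actor's rotation.
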(event Custom|startMov
  (Variables|Default|SetNewVar true))

(event EventBeginPlay)

(event Collision|EventActorBeginOverlap
  (params (OtherActor :type Actor%20Object%20Reference)))

(event EventTick
  (params (DeltaSeconds :type Float%20%28single-precision%29))
  (bind _returnvalue (* DeltaSeconds 3e+02))
  (if (Variables|Default|GetNewVar)
    (Transformation|AddLocalRotation (Variables|Default|GetWheel1) (Math|Rotator|MakeRotator _returnvalue 0.0 0.0) false false)
    (Transformation|AddLocalRotation (Variables|Default|GetWheel2) (Math|Rotator|MakeRotator (* _returnvalue -1.0) 0.0 0.0) false false)
    (Transformation|SetActorLocation (Math|Interpolation|VInterpTo (Transformation|GetActorLocation) (Transformation|GetActorLocation (Variables|Default|Getwaypoint)) DeltaSeconds 1.0) false false)))

(fn ConstructionScript)