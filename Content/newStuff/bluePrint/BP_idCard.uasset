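; ID card pickup actor that shows an interaction indicator and flags itself to BP_ThirdPersonCharacter as a "card" item when the player is in range.
; An outer collision toggles the widget's visibility, while the pickup radius fills or unfills it and sets the character's in-radius state.
; Tick refreshes the player reference and turns the indicator toward the camera.
; BeginPlay restricts a SceneCapture2D to render only TempCube.
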(event OnComponentBeginOverlap(showIndicatorCollison)
  (params (OverlappedComponent :type Primitive%20Component%20Object%20Reference) (OtherActor :type Actor%20Object%20Reference) (OtherComp :type Primitive%20Component%20Object%20Reference) (OtherBodyIndex :type Integer) (bFromSweep :type Boolean) (SweepResult :type Hit%20Result%20Structure%20%28by%20ref%29))
  (if (== OtherActor (Variables|Default|GetPC))
    (Development|SetHiddeninGame (Variables|Default|GetitemIndicator) false false)))

(event OnComponentEndOverlap(showIndicatorCollison)
  (params (OverlappedComponent :type Primitive%20Component%20Object%20Reference) (OtherActor :type Actor%20Object%20Reference) (OtherComp :type Primitive%20Component%20Object%20Reference) (OtherBodyIndex :type Integer))
  (if (== (Variables|Default|GetPC) OtherActor)
    (Development|SetHiddeninGame (Variables|Default|GetitemIndicator) true false)))

(event OnComponentBeginOverlap(pickupItemradius)
  (params (OverlappedComponent :type Primitive%20Component%20Object%20Reference) (OtherActor :type Actor%20Object%20Reference) (OtherComp :type Primitive%20Component%20Object%20Reference) (OtherBodyIndex :type Integer) (bFromSweep :type Boolean) (SweepResult :type Hit%20Result%20Structure%20%28by%20ref%29))
  (if (== (Variables|Default|GetPC) OtherActor)
    (bind _aswbp_interact_indicator (Utilities|Casting|CastToWBP_interactIndicator (UserInterface|GetUserWidgetObject (Variables|Default|GetitemIndicator))))
    (Default|FillWidget _aswbp_interact_indicator)
    (CallFunction|PickupRadiusTrue)))

(event OnComponentEndOverlap(pickupItemradius)
  (params (OverlappedComponent :type Primitive%20Component%20Object%20Reference) (OtherActor :type Actor%20Object%20Reference) (OtherComp :type Primitive%20Component%20Object%20Reference) (OtherBodyIndex :type Integer))
  (if (== (Variables|Default|GetPC) OtherActor)
    (bind _aswbp_interact_indicator (Utilities|Casting|CastToWBP_interactIndicator (UserInterface|GetUserWidgetObject (Variables|Default|GetitemIndicator))))
    (Default|UnfillWidget _aswbp_interact_indicator)
    (CallFunction|PickupRadiusFalse)))

(event Custom|pickupRadiusFalse
  (bind _asbp_third_person_character (Utilities|Casting|CastToBP_ThirdPersonCharacter (Variables|Default|GetPC)))
  (Variables|/Game/ThirdPerson/Blueprints/BP_ThirdPersonCharacter.BP_ThirdPersonCharacter_C|SetinItemRadius _asbp_third_person_character false))

(event Custom|pickupRadiusTrue
  (bind _asbp_third_person_character (Utilities|Casting|CastToBP_ThirdPersonCharacter (Variables|Default|GetPC)))
  (Variables|/Game/ThirdPerson/Blueprints/BP_ThirdPersonCharacter.BP_ThirdPersonCharacter_C|SetinItemRadius _asbp_third_person_character true)
  (Variables|/Game/ThirdPerson/Blueprints/BP_ThirdPersonCharacter.BP_ThirdPersonCharacter_C|SetitempickupType _asbp_third_person_character "\"card\""))

(event EventBeginPlay
  (Development|SetHiddeninGame (Variables|Default|GetitemIndicator) true false)
  (Rendering|SceneCapture|ShowOnlyComponent (Variables|Default|GetSceneCaptureComponent2D) (Variables|Default|GettempCube)))

(event Collision|EventActorBeginOverlap
  (params (OtherActor :type Actor%20Object%20Reference)))

(event EventTick
  (params (DeltaSeconds :type Float%20%28single-precision%29))
  (Variables|Default|SetPC (Game|GetPlayerCharacter 0))
  (Transformation|SetWorldRotation (Variables|Default|GetitemIndicator) (Math|Rotator|FindLookatRotation (Transformation|GetWorldLocation (Variables|Default|GetitemIndicator)) (Transformation|GetWorldLocation (Variables|/Script/Engine.PlayerCameraManager|GetTransformComponent (Game|GetPlayerCameraManager 0)))) false false))

(fn ConstructionScript)