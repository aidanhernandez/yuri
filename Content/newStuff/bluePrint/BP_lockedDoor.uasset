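; Locked door actor that opens with a "key" item from the player's inventory, then toggles open and closed once unlocked.
; An overlap radius sets the character's InDoorRadius tag, while the openDoor event searches the inventory and empties the key slot.
; Unlocking plays a bound Level Sequence with the camera blended to the door and player hidden and input-disabled.
; Timelines drive the door's yaw for swinging, or a slight nudge when no key is found.
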(event OnComponentBeginOverlap(openDoorRadius)
  (params (OverlappedComponent :type Primitive%20Component%20Object%20Reference) (OtherActor :type Actor%20Object%20Reference) (OtherComp :type Primitive%20Component%20Object%20Reference) (OtherBodyIndex :type Integer) (bFromSweep :type Boolean) (SweepResult :type Hit%20Result%20Structure%20%28by%20ref%29))
  (bind _asbp_third_person_character (Utilities|Casting|CastToBP_ThirdPersonCharacter OtherActor))
  (Variables|/Game/ThirdPerson/Blueprints/BP_ThirdPersonCharacter.BP_ThirdPersonCharacter_C|SetinDoorRadius _asbp_third_person_character "\"lockedDoor\""))

(event OnComponentEndOverlap(openDoorRadius)
  (params (OverlappedComponent :type Primitive%20Component%20Object%20Reference) (OtherActor :type Actor%20Object%20Reference) (OtherComp :type Primitive%20Component%20Object%20Reference) (OtherBodyIndex :type Integer))
  (bind _asbp_third_person_character (Utilities|Casting|CastToBP_ThirdPersonCharacter OtherActor))
  (Variables|/Game/ThirdPerson/Blueprints/BP_ThirdPersonCharacter.BP_ThirdPersonCharacter_C|SetinDoorRadius _asbp_third_person_character "\"none\""))

(event Custom|openDoor
  (bind _returnvalue (Game|GetPlayerCharacter 0))
  (bind _returnvalue_2 (Game|GetPlayerCharacter 0))
  (if (Variables|Default|GetdoorLocked)
    (bind _asbp_third_person_character (Utilities|Casting|CastToBP_ThirdPersonCharacter (Game|GetPlayerCharacter 0)))
    (bind (_array_element _array_index) (Utilities|Array|ForEachLoopwithBreak (Variables|/Game/ThirdPerson/Blueprints/BP_ThirdPersonCharacter.BP_ThirdPersonCharacter_C|GetinventoryMain _asbp_third_person_character) :!label _label)
      (:LoopBody
        (if (Utilities|String|Contains _array_element "\"key\"")
          (Variables|Default|SetkeyFound true)
          (goto _label Break)
          (else
            (Variables|Default|SetkeyFound false))))
      (:Completed
        (if (Variables|Default|GetkeyFound)
          (Utilities|Array|SetArrayElem (Variables|/Game/ThirdPerson/Blueprints/BP_ThirdPersonCharacter.BP_ThirdPersonCharacter_C|GetinventoryMain _asbp_third_person_character) _array_index "\"empty\"")
          (bind (_outactor _returnvalue_3) (Sequencer|Player|CreateLevelSequencePlayer "/Game/sequences/openDoor.openDoor"))
          (Class|LevelSequenceActor|AddBinding _outactor (|GetSequenceBinding) self false)
          (Game|Player|SetViewTargetwithBlend (Game|GetPlayerController 0) self 0.5 "VTBlend_Linear" 0.0 false)
          (Input|DisableInput _returnvalue_2 (Game|GetPlayerController 0))
          (Rendering|SetActorHiddenInGame _returnvalue_2 true)
          (bind _asbp_third_person_character_2 (Utilities|Casting|CastToBP_ThirdPersonCharacter _returnvalue_2))
          (Variables|/Game/ThirdPerson/Blueprints/BP_ThirdPersonCharacter.BP_ThirdPersonCharacter_C|SetcameraShakeDisabled _asbp_third_person_character_2 true)
          (Development|SetHiddeninGame (Variables|Default|GetKey) false false)
          (Sequencer|Player|Play _returnvalue_3 :!class /Script/MovieScene.MovieSceneSequencePlayer)
          (Utilities|FlowControl|Delay (Class|TimeManagementBlueprintLibrary|ToSeconds(QualifiedFrameTime) (Media|MediaPlayer|GetDuration _returnvalue_3)))
          (bind _doorfloat (Timeline|Timeline_0 PlayFromStart)
            (:Update
              (Transformation|SetRelativeRotation (Variables|Default|Getdoor) (Math|Rotator|MakeRotator 0.0 0.0 (Math|Float|Lerp 0.0 -9e+01 _doorfloat)) false false)
              (Variables|Default|SetdoorOpen? true)
              (Utilities|FlowControl|Delay 0.2)
              (Game|Player|SetViewTargetwithBlend (Game|GetPlayerController 0) (Game|GetPlayerCharacter 0) 0.5 "VTBlend_Linear" 0.0 false)
              (Utilities|FlowControl|Delay 0.1)
              (Development|SetHiddeninGame (Variables|Default|GetKey) true false)
              (Variables|Default|SetdoorLocked false)
              (Input|EnableInput _returnvalue (Game|GetPlayerController 0))
              (Rendering|SetActorHiddenInGame _returnvalue false)
              (bind _asbp_third_person_character_3 (Utilities|Casting|CastToBP_ThirdPersonCharacter _returnvalue))
              (Variables|/Game/ThirdPerson/Blueprints/BP_ThirdPersonCharacter.BP_ThirdPersonCharacter_C|SetcameraShakeDisabled _asbp_third_person_character_3 false)))
          (else
            (bind _doorfloat_2 (Timeline|Timeline_2 PlayFromStart)
              (:Finished
                (Transformation|SetRelativeRotation (Variables|Default|Getdoor) (Math|Rotator|MakeRotator 0.0 0.0 (Math|Float|Lerp 0.0 -1.0 _doorfloat_2)) false false)
                (bind _doorfloat_3 (Timeline|Timeline_3 ReverseFromEnd)
                  (:Finished
                    (Transformation|SetRelativeRotation (Variables|Default|Getdoor) (Math|Rotator|MakeRotator 0.0 0.0 (Math|Float|Lerp 0.0 -1.0 _doorfloat_3)) false false)))))))))
    (elif (Variables|Default|GetdoorOpen?)
      (bind _doorfloat_4 (Timeline|Timeline ReverseFromEnd)
        (:Update
          (Transformation|SetRelativeRotation (Variables|Default|Getdoor) (Math|Rotator|MakeRotator 0.0 0.0 (Math|Float|Lerp 0.0 -9e+01 _doorfloat_4)) false false)
          (Variables|Default|SetdoorOpen? false)))
      (else
        (bind _doorfloat_5 (Timeline|Timeline_1 PlayFromStart)
          (:Update
            (Transformation|SetRelativeRotation (Variables|Default|Getdoor) (Math|Rotator|MakeRotator 0.0 0.0 (Math|Float|Lerp 0.0 -9e+01 _doorfloat_5)) false false)
            (Variables|Default|SetdoorOpen? true)))))))

(fn ConstructionScript)