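; BP_ammoBox is an ammo box pickup that notifies the third-person character when it enters or leaves the box's mesh overlap.
; Begin overlap calls AmmoBoxCollison on the character with the box as actor, unless the box is already used; end overlap always sends the exit call.
; The ammoUsed event swaps the mesh to an empty box, sets the used flag NewVar and clears InAmmoBox on player character 0.
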(event OnComponentBeginOverlap(StaticMesh)
  (params (OverlappedComponent :type Primitive%20Component%20Object%20Reference) (OtherActor :type Actor%20Object%20Reference) (OtherComp :type Primitive%20Component%20Object%20Reference) (OtherBodyIndex :type Integer) (bFromSweep :type Boolean) (SweepResult :type Hit%20Result%20Structure%20%28by%20ref%29))
  (if (not (Variables|Default|GetNewVar))
    (bind _asbp_third_person_character (Utilities|Casting|CastToBP_ThirdPersonCharacter OtherActor))
    (Default|AmmoBoxCollison _asbp_third_person_character true self)))

(event OnComponentEndOverlap(StaticMesh)
  (params (OverlappedComponent :type Primitive%20Component%20Object%20Reference) (OtherActor :type Actor%20Object%20Reference) (OtherComp :type Primitive%20Component%20Object%20Reference) (OtherBodyIndex :type Integer))
  (bind _asbp_third_person_character (Utilities|Casting|CastToBP_ThirdPersonCharacter OtherActor))
  (Default|AmmoBoxCollison _asbp_third_person_character false self))

(event Custom|ammoUsed
  (Components|StaticMesh|SetStaticMesh (Variables|Default|GetStaticMesh) "/Game/newStuff/importedStuff/FINALOBJ/ammoBox/ammoBOXnoAmov3.ammoBOXnoAmov3")
  (Variables|Default|SetNewVar true)
  (bind _asbp_third_person_character (Utilities|Casting|CastToBP_ThirdPersonCharacter (Game|GetPlayerCharacter 0)))
  (Variables|/Game/ThirdPerson/Blueprints/BP_ThirdPersonCharacter.BP_ThirdPersonCharacter_C|SetinAmmoBox _asbp_third_person_character false))

(fn ConstructionScript)