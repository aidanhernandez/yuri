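; Interactive nightstand with two drawers that can each hold an item, either a herb or a slug.
; BeginPlay sets each item's mesh from its string variable, and box overlaps tell the third-person character when it enters or leaves range.
; The drawers event picks bottom when crouching, top otherwise: closed drawers slide open via timelines.
; Open drawers pass any item to the character, or slide shut when marked empty.
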(event OnComponentBeginOverlap(Box)
  (params (OverlappedComponent :type Primitive%20Component%20Object%20Reference) (OtherActor :type Actor%20Object%20Reference) (OtherComp :type Primitive%20Component%20Object%20Reference) (OtherBodyIndex :type Integer) (bFromSweep :type Boolean) (SweepResult :type Hit%20Result%20Structure%20%28by%20ref%29))
  (bind _asbp_third_person_character (Utilities|Casting|CastToBP_ThirdPersonCharacter OtherActor))
  (Default|NightStandCollision _asbp_third_person_character true self))

(event OnComponentEndOverlap(Box)
  (params (OverlappedComponent :type Primitive%20Component%20Object%20Reference) (OtherActor :type Actor%20Object%20Reference) (OtherComp :type Primitive%20Component%20Object%20Reference) (OtherBodyIndex :type Integer))
  (bind _asbp_third_person_character (Utilities|Casting|CastToBP_ThirdPersonCharacter OtherActor))
  (Default|NightStandCollision _asbp_third_person_character false self))

(event Custom|drawers
  (params (crouching? :type Boolean))
  (if crouching?
    (CallFunction|BottomDrawerStuff)
    (elif (Variables|Default|GetareOpen)
      (if (not (Utilities|Enum|Equal(Enum) (Variables|Default|GetitemTopDrawer) "\"empty\""))
        (bind _asbp_third_person_character (Utilities|Casting|CastToBP_ThirdPersonCharacter (Game|GetPlayerCharacter 0)))
        (Default|ItemfromDrawer _asbp_third_person_character (Variables|Default|GetitemTopDrawer) self false)
        (else
          (bind _newtrack_0 (Timeline|Timeline_0 PlayFromStart)
            (:Update
              (Transformation|SetRelativeLocation (Variables|Default|GettopDrawer) (.location (Math|Transform|Lerp(Transform) (Math|Transform|MakeTransform "0, 0, 0" "0, 0, 0" "1.000000,1.000000,1.000000") (Math|Transform|MakeTransform "60.000000,0.000000,0.000000" "0, 0, 0" "1.000000,1.000000,1.000000") _newtrack_0)) false false)
              (Variables|Default|SetareOpen false)))))
      (else
        (bind _newtrack_0_2 (Timeline|Timeline PlayFromStart)
          (:Update
            (Transformation|SetRelativeLocation (Variables|Default|GettopDrawer) (.location (Math|Transform|Lerp(Transform) (Math|Transform|MakeTransform "0, 0, 0" "0, 0, 0" "1.000000,1.000000,1.000000") (Math|Transform|MakeTransform "60.000000,0.000000,0.000000" "0, 0, 0" "1.000000,1.000000,1.000000") _newtrack_0_2)) false false)
            (Variables|Default|SetareOpen true)))))))

(event Custom|bottomDrawerStuff
  (if (Variables|Default|GetareOpenB)
    (if (not (Utilities|Enum|Equal(Enum) (Variables|Default|GetitembottomDrawer) "\"empty\""))
      (bind _asbp_third_person_character (Utilities|Casting|CastToBP_ThirdPersonCharacter (Game|GetPlayerCharacter 0)))
      (Default|ItemfromDrawer _asbp_third_person_character (Variables|Default|GetitembottomDrawer) self true)
      (else
        (bind _newtrack_0 (Timeline|Timeline_2 PlayFromStart)
          (:Update
            (Transformation|SetRelativeLocation (Variables|Default|GetbottomDrawer) (.location (Math|Transform|Lerp(Transform) (Math|Transform|MakeTransform "5.000000,0.000000,0.000000" "0, 0, 0" "1.000000,1.000000,1.000000") (Math|Transform|MakeTransform "60.000000,0.000000,0.000000" "0, 0, 0" "1.000000,1.000000,1.000000") _newtrack_0)) false false)
            (Variables|Default|SetareOpenB false)))))
    (else
      (bind _newtrack_0_2 (Timeline|Timeline_1 PlayFromStart)
        (:Update
          (Transformation|SetRelativeLocation (Variables|Default|GetbottomDrawer) (.location (Math|Transform|Lerp(Transform) (Math|Transform|MakeTransform "5.000000,0.000000,0.000000" "0, 0, 0" "1.000000,1.000000,1.000000") (Math|Transform|MakeTransform "60.000000,0.000000,0.000000" "0, 0, 0" "1.000000,1.000000,1.000000") _newtrack_0_2)) false false)
          (Variables|Default|SetareOpenB true))))))

(event EventTick
  (params (DeltaSeconds :type Float%20%28single-precision%29)))

(event EventBeginPlay
  (bind _staticmesh1 (Variables|Default|GetStaticMesh1))
  (Utilities|FlowControl|Sequence
    (:then_0
      (switch string (Variables|Default|GetitemTopDrawer)
        (:"herb"
          (Components|StaticMesh|SetStaticMesh (Variables|Default|GetStaticMesh) "/Game/newStuff/importedStuff/FINALOBJ/plant/Plance.Plance")
          (Transformation|SetRelativeTransform (Variables|Default|GetStaticMesh) (Math|Transform|MakeTransform "10.000000,0.000000,10.000000" "0, 0, 0" "0.150000,0.150000,0.150000") false false))
        (:"slug"
          (Components|StaticMesh|SetStaticMesh (Variables|Default|GetStaticMesh) "/Game/newStuff/importedStuff/slugbert.slugbert")
          (Transformation|SetRelativeTransform (Variables|Default|GetStaticMesh) (Math|Transform|MakeTransform "10.000000,0.000000,30.000000" "0.000000,90.000000,0.000000" "0.150000,0.150000,0.150000") false false))))
    (:then_1
      (switch string (Variables|Default|GetitembottomDrawer)
        (:"herb"
          (Components|StaticMesh|SetStaticMesh _staticmesh1 "/Game/newStuff/importedStuff/FINALOBJ/plant/Plance.Plance")
          (Transformation|SetRelativeTransform _staticmesh1 (Math|Transform|MakeTransform "10.000000,0.000000,-70.000000" "0, 0, 0" "0.150000,0.150000,0.150000") false false))
        (:"slug"
          (Components|StaticMesh|SetStaticMesh _staticmesh1 "/Game/newStuff/importedStuff/slugbert.slugbert")
          (Transformation|SetRelativeTransform _staticmesh1 (Math|Transform|MakeTransform "10.000000,0.000000,-70.000000" "0.000000,90.000000,0.000000" "0.150000,0.150000,0.150000") false false))))))

(fn ConstructionScript)